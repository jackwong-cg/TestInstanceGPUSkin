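; Actor Blueprint that displays an adjustable number of mesh instances through its InstanceStaticMesh component.
; ChangeCount clears all instances, then rebuilds them in world space using per-index transforms from GetInstTransform.
; The requested count is capped at GenerateCount and stored in VisableCount, which becomes zero for non-positive requests.
; Its event graph and construction script are empty.
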(event EventBeginPlay)

(event Collision|EventActorBeginOverlap
  (params (OtherActor :type Actor%20Object%20Reference)))

(event EventTick
  (params (DeltaSeconds :type Float%20%28single-precision%29)))

(fn ConstructionScript)

(fn ChangeCount
  (params (count :type Integer))
  (bind _generatecount (Variables|Default|GetGenerateCount))
  (bind _returnvalue (Math|Integer|Min(Integer) count _generatecount))
  (Components|InstancedStaticMesh|ClearInstances (Variables|Default|GetinstanceStaticMesh))
  (if (> count 0)
    (for _index (range 0 _returnvalue)
      (bind _returnvalue_2 (Class|InstanceSkeletelMeshActor|GetInstTransform _index))
      (Class|InstancedStaticMeshComponent|AddInstanceWorldSpace (Variables|Default|GetinstanceStaticMesh) _returnvalue_2))
    (Variables|Default|SetVisableCount _returnvalue)
    (else
      (Variables|Default|SetVisableCount 0))))