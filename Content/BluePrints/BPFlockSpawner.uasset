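; BPFlockSpawner is an actor Blueprint for laying out grids of static mesh instances, but nothing currently triggers the spawning.
; SpawnInst uses nested loops to add evenly spaced world-space instances to a given instanced mesh component, adding only the actor's height to the offset.
; Three unconnected calls would place the LOD0, LOD1 and LOD2 components' grids side by side along Y.
; BeginPlay, Tick and the construction script are empty.
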(event EventBeginPlay)

(event Collision|EventActorBeginOverlap
  (params (OtherActor :type Actor%20Object%20Reference)))

(event EventTick
  (params (DeltaSeconds :type Float%20%28single-precision%29)))

(fn ConstructionScript)

(fn SpawnInst
  (params (Offset :type Vector) (MeshLod :type Instanced%20Static%20Mesh%20Component%20Object%20Reference))
  (for _index (range 0 5)
    (for _index_2 (range 0 5)
      (Class|InstancedStaticMeshComponent|AddInstanceWorldSpace MeshLod (Math|Transform|MakeTransform (Math|Vector|MakeVector (+ (.x Offset) (* _index 3e+01)) (+ (.y Offset) (* _index_2 3e+01)) (+ (.z Offset) (.z (Transformation|GetActorLocation)))) "0, 0, 0" "1,1,1")))))